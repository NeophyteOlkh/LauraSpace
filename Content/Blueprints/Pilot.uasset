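; Player pilot pawn for a shooter, with sideways axis movement, three hit points and score tracking.
; Shooting spawns a projectile from a scene component only while no previous one is valid; losing all HP opens NewMap.
; Tick projects its position to screen space to set edge-stop flags, which the movement here never reads.
; Helpers restore HP up to the cap and award miss-penalized points; EnemyDead and Count are empty.
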(event Custom|Damage
  ;[1 1 1] Дамаг
  (Variables|Default|SetHP (- (Variables|Default|GetHP) 1))
  (if (== (Variables|Default|GetHP) 0)
    (CallFunction|GameOver)))

(event Custom|GameOver
  (Game|OpenLevel(byName) "NewMap"))

(event EventBeginPlay
  (Variables|Default|SetPlaceOfSpawn (Utilities|Array|MakeArray (Variables|Default|GetScene)))
  (Variables|Default|SetHP 3))

(event EventTick
  (params (DeltaSeconds :type Float%20%28single-precision%29))
  (bind _returnvalue (Transformation|GetActorLocation))
  (bind _returnvalue_2 (Game|GetPlayerController 0))
  (bind _returnvalue_3 (Viewport|GetViewportSize))
  (bind _margin (Variables|Default|GetMargin))
  (bind _margin_2 (Variables|Default|GetMargin))
  (bind _screenposition (Class|GameplayStatics|ProjectWorldtoScreen _returnvalue_2 _returnvalue false))
  (bind (_x _y) (Math|Vector2D|BreakVector2D _returnvalue_3))
  (bind (_x_2 _y_2) (Math|Vector2D|BreakVector2D _screenposition))
  (Utilities|FlowControl|Sequence
    (:then_0
      (Variables|Default|SetStop%20Left (< _x_2 _margin_2)))
    (:then_1
      (Variables|Default|SetStop%20Right (> _x_2 (- _x _margin_2))))
    (:then_2
      (Variables|Default|SetStop%20Up (< _y_2 _margin)))
    (:then_3
      (Variables|Default|SetStop%20down (> _y_2 (- _y _margin))))))

(event Input|ActionEvents|InputActionShooting
  (params (Key :type Key%20Structure :default "None"))
  (bind _placeofspawn (Variables|Default|GetPlaceOfSpawn))
  (bind _output (Utilities|Array|Get(acopy) _placeofspawn))
  (bind _returnvalue (Transformation|GetWorldTransform _output))
  ;[1 1 1] Стрельба
  (:Pressed
    (Utilities|IsValid (stale _returnvalue_2)
      (:Is%20Not%20Valid
        (bind _returnvalue_2 (Game|SpawnActorfromClass "/Game/Blueprints/Projectyle1.Projectyle1_C" (Math|Transform|MakeTransform (.location _returnvalue) (.rotation _returnvalue) (.scale _returnvalue)) "Undefined" 0 0))))))

(event Input|AxisEvents|InputAxisMovementLeft
  (params (AxisValue :type Float%20%28single-precision%29))
  ;[1 1 1] Перемещение
  (Transformation|AddActorWorldOffset (Math|Vector|MakeVector 0.0 AxisValue 0.0)))

(fn ConstructionScript)

(fn EnemyDead)

(fn Count)

(fn Lifes
  (Variables|Default|SetHP (Math|Integer|Min(Integer) (+ (Variables|Default|GetHP) 1) 3)))

(fn +Score
  (Variables|Default|SetScore (+ (Variables|Default|GetScore) (- 100 (* 5 (Math|Integer|Min(Integer) 10 (Variables|Default|GetMiss)))))))