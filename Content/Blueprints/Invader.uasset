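; Invader is an enemy actor that marches in a repeating zigzag, fires projectiles at random and is destroyed by its TakeDamage event.
; Four chained timelines loop the movement, using delta-scaled world offsets to alternate opposite Y sweeps with steps along negative X.
; A looping timer with a randomized start delay gives a chance to spawn a ProjectyleEnemy at the Scene component's transform.
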(event Custom|Shoot
  (bind _placeofspawn (Variables|Default|GetPlaceOfSpawn))
  (bind _output (Utilities|Array|Get(acopy) _placeofspawn))
  (bind _returnvalue (Transformation|GetWorldTransform _output))
  (Game|SpawnActorfromClass "/Game/Blueprints/ProjectyleEnemy.ProjectyleEnemy_C" (Math|Transform|MakeTransform (.location _returnvalue) (.rotation _returnvalue) (.scale _returnvalue)) "Undefined" 0 0))

(event Custom|Movement
  (Timeline|Timeline_0 Play
    (:Update
      (Transformation|AddActorWorldOffset (* "0,50.000000, 0" (Utilities|Time|GetWorldDeltaSeconds))))
    (:Finished
      (Timeline|Timeline_1 PlayFromStart
        (:Update
          (Transformation|AddActorWorldOffset (* "-75.000000,0.000000, 0" (Utilities|Time|GetWorldDeltaSeconds))))
        (:Finished
          (Timeline|Timeline_2 PlayFromStart
            (:Update
              (Transformation|AddActorWorldOffset (* "0,-50.000000, 0" (Utilities|Time|GetWorldDeltaSeconds))))
            (:Finished
              (Timeline|Timeline_3 PlayFromStart
                (:Update
                  (Transformation|AddActorWorldOffset (* "-75.000000,0.000000, 0" (Utilities|Time|GetWorldDeltaSeconds))))
                (:Finished
                  (Timeline|Timeline_0 PlayFromStart))))))))))

(event Custom|Try
  (if (< (Math|Random|RandomFloat) 0.25)
    (CallFunction|Shoot)))

(event EventBeginPlay
  (Variables|Default|SetPlaceOfSpawn (Utilities|Array|MakeArray (Variables|Default|GetScene)))
  (CallFunction|Movement)
  (Utilities|Time|SetTimerbyEvent (delegate Custom|Try) 2.0 true 0.0 3.0))

(event EventTakeDamage
  (Actor|DestroyActor))

(fn ConstructionScript)